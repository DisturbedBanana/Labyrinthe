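; AC_LineTrace is an actor component that lets its owner, presumably the player, press buttons in the labyrinth.
; Its CastLineTrace event traces 500 units forward from the owner's camera on a custom trace channel, with debug drawing left on.
; If the hit actor is a BP_Button, it calls ActivateButton on it; any other hit does nothing.
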(event Custom|CastLineTrace
  (bind _output_get (Variables|Default|SetPlayer (Components|GetOwner)))
  (bind _output_get_2 (Variables|Default|SetCamera (Actor|GetComponentbyClass _output_get "/Script/Engine.CameraComponent")))
  (Variables|Default|SetStartLineTraceLocation (Transformation|GetWorldLocation _output_get_2))
  (Variables|Default|SetEndLineTraceLocation (+ (Transformation|GetWorldLocation _output_get_2) (* (Math|Vector|GetForwardVector (Transformation|GetWorldRotation _output_get_2)) (Math|Conversions|ToVector(Float) 5e+02))))
  (bind _outhit (Collision|LineTraceByChannel (Variables|Default|GetStartLineTraceLocation) (Variables|Default|GetEndLineTraceLocation) "TraceTypeQuery3" false 0 "ForDuration"))
  (bind _asbp_button (Utilities|Casting|CastToBP_Button (.HitActor (Collision|BreakHitResult _outhit))))
  (Default|ActivateButton _asbp_button))