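; BP_Torche is an interactable torch in the labyrinth that the player lights or puts out while standing near it.
; SwitchTorchState, triggered by the E key, toggles the fire particle and active flag only when the player is present, as set by BP_Collision through ChangePlayerPresence.
; Each toggle adds or subtracts one from the game mode's secret-opening condition; the fire starts deactivated on BeginPlay.
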(event Custom|ChangePlayerPresence
  (params (value :type Boolean))
  ;[1 1 1] Switches if the torch can be activated (depends on player proximity - triggerred by BP_Collision)
  (Variables|Default|SetisPlayerHere value))

(event Custom|SwitchTorchState
  ;[1 1 1] Switches the torch state (Depends if the torch is already active or not - triggered by keybind E)
  (if (Variables|Default|GetisTorchActive)
    (if (Variables|Default|GetisPlayerHere)
      (Components|Activation|Deactivate (Variables|Default|GetP_Fire))
      (Variables|Default|SetisTorchActive false)
      (bind _asbp_first_person_game_mode (Utilities|Casting|CastToBP_FirstPersonGameMode (Game|GetGameMode)))
      (Default|ChangeSecretOpeningCondition _asbp_first_person_game_mode -1))
    (elif (Variables|Default|GetisPlayerHere)
      (Components|Activation|Activate (Variables|Default|GetP_Fire) false)
      (Variables|Default|SetisTorchActive true)
      (bind _asbp_first_person_game_mode_2 (Utilities|Casting|CastToBP_FirstPersonGameMode (Game|GetGameMode)))
      (Default|ChangeSecretOpeningCondition _asbp_first_person_game_mode_2 1))))

(event EventBeginPlay
  ;[1 1 1] Deactivates torch on game start
  (Components|Activation|Deactivate (Variables|Default|GetP_Fire)))

(fn ConstructionScript)