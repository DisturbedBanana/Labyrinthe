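; BP_Button is a toggle button in the labyrinth that counts toward opening a secret door.
; ActivateButton flips IsActivated and instantly moves the Button component a short distance down or up along its up vector, with sweep.
; Each toggle tells BP_FirstPersonGameMode via ChangeSecretOpeningCondition to add or remove one from the door's opening condition, so the game mode manages the door.
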(event Custom|ActivateButton
  (bind _button (Variables|Default|GetButton))
  (bind _button_2 (Variables|Default|GetButton))
  ;[1 1 1] Checks if button is already pushed down
  (if (Variables|Default|GetisActivated)
    ;[1 1 1] Button is already activated -> push it back up
    (Transformation|SetWorldLocation (Variables|Default|GetButton) (+ (Transformation|GetWorldLocation _button) (* (Math|Vector|GetUpVector _button) (Math|Conversions|ToVector(Float) 9.0))) true false)
    ;[1 1 1] Deactivate it and call the event managing the door
    (Variables|Default|SetisActivated false)
    (bind _asbp_first_person_game_mode (Utilities|Casting|CastToBP_FirstPersonGameMode (Game|GetGameMode)))
    (Default|ChangeSecretOpeningCondition _asbp_first_person_game_mode -1)
    (else
      ;[1 1 1] Button is not activated -> push it down
      (Transformation|SetWorldLocation _button_2 (+ (Transformation|GetWorldLocation _button_2) (* (Math|Vector|GetUpVector _button_2) (Math|Conversions|ToVector(Float) -9.0))) true false)
      ;[1 1 1] Activate it and call the event managing the door
      (Variables|Default|SetisActivated true)
      (bind _asbp_first_person_game_mode_2 (Utilities|Casting|CastToBP_FirstPersonGameMode (Game|GetGameMode)))
      (Default|ChangeSecretOpeningCondition _asbp_first_person_game_mode_2 1))))

(fn ConstructionScript)